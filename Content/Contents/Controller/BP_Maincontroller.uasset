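; BP_Maincontroller is the character input controller, turning Enhanced Input actions into movement, jump and look calls.
; On BeginPlay it adds the MP_Character mapping context to the local player's Enhanced Input subsystem.
; Each action event forwards to its own function for directional movement, jumping or mouse rotation, with those functions defined outside this file.
; A Mouse 2D debug key release also feeds MouseRotation.
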(event Input|EnhancedActionEvents|EnhancedInputActionCh_Back
  (params (ActionValue :type Boolean) (ElapsedSeconds :type Float%20%28double-precision%29) (TriggeredSeconds :type Float%20%28double-precision%29) (InputAction :type Input%20Action%20Object%20Reference :default "/Game/Contents/Controller/Ch_Back.Ch_Back"))
  (Class|MainController|SMoveBack))

(event Input|EnhancedActionEvents|EnhancedInputActionCh_Front
  (params (ActionValue :type Boolean) (ElapsedSeconds :type Float%20%28double-precision%29) (TriggeredSeconds :type Float%20%28double-precision%29) (InputAction :type Input%20Action%20Object%20Reference :default "/Game/Contents/Controller/Ch_Front.Ch_Front"))
  (Class|MainController|WMoveFront))

(event Input|EnhancedActionEvents|EnhancedInputActionCh_Left
  (params (ActionValue :type Boolean) (ElapsedSeconds :type Float%20%28double-precision%29) (TriggeredSeconds :type Float%20%28double-precision%29) (InputAction :type Input%20Action%20Object%20Reference :default "/Game/Contents/Controller/Ch_Left.Ch_Left"))
  (Class|MainController|AMoveLeft))

(event Input|EnhancedActionEvents|EnhancedInputActionCh_Right
  (params (ActionValue :type Boolean) (ElapsedSeconds :type Float%20%28double-precision%29) (TriggeredSeconds :type Float%20%28double-precision%29) (InputAction :type Input%20Action%20Object%20Reference :default "/Game/Contents/Controller/Ch_Right.Ch_Right"))
  (Class|MainController|DMoveRight))

(event Input|EnhancedActionEvents|EnhancedInputActionCh_Jump
  (params (ActionValue :type Boolean) (ElapsedSeconds :type Float%20%28double-precision%29) (TriggeredSeconds :type Float%20%28double-precision%29) (InputAction :type Input%20Action%20Object%20Reference :default "/Game/Contents/Controller/Ch_Jump.Ch_Jump"))
  (:Started
    (Class|MainController|SpaceJump)))

(event Input|EnhancedActionEvents|EnhancedInputActionCh_MouseRotation
  (params (ActionValue :type Vector%202D%20Structure) (ElapsedSeconds :type Float%20%28double-precision%29) (TriggeredSeconds :type Float%20%28double-precision%29) (InputAction :type Input%20Action%20Object%20Reference :default "/Game/Contents/Controller/Ch_MouseRotation.Ch_MouseRotation"))
  (Class|MainController|MouseRotation (stale Input|MouseEvents|DebugKeyMouse2D ActionValue)))

(event EventBeginPlay
  (Input|AddMappingContext (PlayerController|LocalPlayerSubsystems|GetEnhancedInputLocalPlayerSubsystem self) "/Game/Contents/Controller/MP_Character.MP_Character" 0 "(bIgnoreAllPressedKeysUntilRelease=True,bForceImmediately=False,bNotifyUserSettings=False)"))

(event EventTick
  (params (DeltaSeconds :type Float%20%28single-precision%29)))

(event Input|MouseEvents|DebugKeyMouse2D
  (params (Key :type Key%20Structure :default "None") (ActionValue :type Input%20Action%20Value%20Structure))
  (:Released
    (Class|MainController|MouseRotation ActionValue)))

(fn ConstructionScript)